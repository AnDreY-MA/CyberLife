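; GA_Sprint is the sprint gameplay ability, applying a stamina effect to the owner while active.
; On activation it async-loads and applies that effect, storing the handle, and watches for an attribute falling to or below a threshold to end itself.
; When the ability ends, it removes the effect by handle and tries to activate abilities tagged Abilities.RegenStamina.
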(event Ability|EventActivateAbility
  (|CallParentFunction)
  (Ability|Tasks|WaitForAttributeChangeWithComparison :InAttribute "(AttributeName=\"Stamina\",Attribute=/Script/CyberLife.CharacterAttributeSet:Stamina,AttributeOwner=\"/Script/CoreUObject.Class'/Script/CyberLife.CharacterAttributeSet'\")" :InComparisonType "LessThanOrEqualTo" :OptionalExternalOwner 0
    (:then
      (|ApplyStaminaEffect))
    (:OnChange
      (Ability|EndAbility))))

(event Ability|EventOnEndAbility
  (params (bWasCancelled :type Boolean))
  (|CallParentFunction bWasCancelled)
  (Ability|RemoveGameplayEffectFromOwnerWithHandle (Variables|Default|GetStaminaHandle))
  (Abilities|TryActivateAbilitiesbyTag (Ability|GetAbilitySystemComponentfromActorInfo) (GameplayTags|MakeGameplayTagContainerfromTag "(TagName=\"Abilities.RegenStamina\")") true))