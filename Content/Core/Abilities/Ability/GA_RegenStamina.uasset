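; Gameplay ability that regenerates stamina by applying a regen Gameplay Effect to its owner.
; On activation it async-loads the effect class, applies it and stores the handle.
; An attribute-change task then ends the ability when the watched value exactly equals an attribute base value read right after the effect is applied.
; Ending the ability removes the effect by its handle and clears the task reference.
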(event Ability|EventActivateAbility
  (Utilities|AsyncLoadClassAsset (Variables|Default|GetRegenEffect)
    (:Completed
      (bind _returnvalue (Ability|ApplyGameplayEffectToOwner (Utilities|ResolveSoftReference (Variables|Default|GetRegenEffect))))
      (Variables|Default|SetEffectHandle _returnvalue)
      (bind _asynctaskproxy (Ability|Tasks|WaitForAttributeChangeWithComparison :InAttribute "(AttributeName=\"Health\",Attribute=/Script/CyberLife.CharacterAttributeSet:Health,AttributeOwner=\"/Script/CoreUObject.Class'/Script/CyberLife.CharacterAttributeSet'\")" :InComparisonType "ExactlyEqualTo" :InComparisonValue (.ReturnValue (Class|AbilitySystemBlueprintLibrary|GetFloatAttributeBasefromAbilitySystemComponent (Ability|GetAbilitySystemComponentfromActorInfo) "(AttributeName=\"MaxHealth\",Attribute=/Script/CyberLife.CharacterAttributeSet:MaxHealth,AttributeOwner=\"/Script/CoreUObject.Class'/Script/CyberLife.CharacterAttributeSet'\")")) :OptionalExternalOwner 0)
        (:then
          (Variables|Default|SetChangeTask _asynctaskproxy))
        (:OnChange
          (Ability|EndAbility))))))

(event Ability|EventOnEndAbility
  (params (bWasCancelled :type Boolean))
  (Ability|RemoveGameplayEffectFromOwnerWithHandle (Variables|Default|GetEffectHandle))
  (Variables|Default|SetChangeTask 0))