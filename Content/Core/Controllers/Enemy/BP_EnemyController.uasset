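; Enemy AI controller that turns sight, hearing and damage perception into enemy reactions.
; On each perception update, it checks every updated actor with CanSenseActor for all three senses.
; Sight passes the actor to its handler, hearing passes the stimulus location, and damage starts investigating that location with a debug print.
; BPCanSenseActor implements a Blueprint stimulus lookup by sense class, but the event graph does not call it.
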(event OnPerceptionUpdated(EnemyPerceptionComponent)
  (params (UpdatedActors :type Array%20of%20Actor%20Object%20References))
  (for _array_element UpdatedActors
    (Utilities|FlowControl|Sequence
      (:then_0
        (bind _returnvalue (Class|EnemyControllerBase|CanSenseActor _array_element "Sight"))
        (if _returnvalue
          (Class|EnemyControllerBase|HandleSensedSight _array_element)))
      (:then_1
        (bind (_outstimulus _returnvalue_2) (Class|EnemyControllerBase|CanSenseActor _array_element "Hearing"))
        (if _returnvalue_2
          (Class|EnemyControllerBase|HandleSensedSound (.StimulusLocation (Utilities|Struct|BreakAIStimulus _outstimulus)))))
      (:then_2
        (bind (_outstimulus_2 _returnvalue_3) (Class|EnemyControllerBase|CanSenseActor _array_element "Damaging"))
        (if _returnvalue_3
          (Class|EnemyControllerBase|SetStateasInvestigating (.StimulusLocation (Utilities|Struct|BreakAIStimulus _outstimulus_2)))
          (Development|PrintString "Hello"))))))

(fn ConstructionScript)

(fn BPCanSenseActor
  (params (Actor :type Actor%20Object%20Reference) (SenseState :type EAISenseState%20Enum :default "None"))
  (bind _info (Class|AIPerceptionComponent|GetActorsPerception (Variables|Default|GetEnemyPerceptionComponent) Actor))
  (for _array_element (.LastSensedStimuli (Utilities|Struct|BreakActorPerceptionBlueprintInfo _info))
    (bind _returnvalue (Class|AIPerceptionSystem|GetSenseClassforStimulus _array_element))
    (if (== _returnvalue (Utilities|Select :Index SenseState :None 0 :Sight "/Script/AIModule.AISense_Sight" :Hearing "/Script/AIModule.AISense_Hearing" :Damaging "/Script/AIModule.AISense_Damage"))
      (return (.bSuccessfullySensed (Utilities|Struct|BreakAIStimulus _array_element)) _array_element))))