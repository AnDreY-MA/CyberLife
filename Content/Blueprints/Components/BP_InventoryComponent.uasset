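; BP_InventoryComponent is a grid inventory component that fits multi-tile items into free space.
; OnAddItem calls TryAddItem, which scans slot indices for space and places the item at the first fit.
; If none fits, a DoOnce rotates the item and repeats the scan before reporting failure.
; The BPForEachIndex macro iterates every tile an item's dimensions cover from its top-left index.
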(event EventOnAddItem
  (params (Item :type Item%20Object%20Object%20Reference))
  (CallFunction|TryAddItem Item))

(fn TryAddItem
  (params (ItemObject :type Item%20Object%20Object%20Reference))
  (Utilities|IsValid ItemObject
    (:Is%20Valid
      (for (_ _array_index) (Variables|Default|GetItems) :!label _label
        (bind _returnvalue (Class|InventoryComponent|IsSpaceAvailable ItemObject _array_index))
        (if _returnvalue
          (Class|InventoryComponent|AddItemat ItemObject _array_index)
          (return true)))
      (Utilities|FlowControl|Sequence
        (:then_0
          (Utilities|FlowControl|DoOnce false
            (:Completed
              (Class|ItemObject|Rotate ItemObject)
              (goto _label))))
        (:then_1
          (return false))))))