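; BP_MyGameStateBase is a game state Blueprint that provides a function for spawning an item object into the world in front of a given actor.
; The spawn point sits a set distance along the actor's forward vector, optionally snapped to the ground by a downward Visibility line trace.
; It spawns the class supplied by the item object, then passes that object to the new actor.
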(fn ConstructionScript)

(fn BPSpawnItemfromActor
  (params (ItemObject :type Item%20Object%20Object%20Reference) (Actor :type Actor%20Object%20Reference) (GroundClamp :type Boolean))
  (Utilities|FlowControl|Sequence
    (:then_0
      (LocalVariables|SetSpawnLocation (+ (Transformation|GetActorLocation Actor) (* (Transformation|GetActorForwardVector Actor) (Variables|Default|GetBPDistanceSpawn))))
      (if GroundClamp
        (bind (_outhit _returnvalue) (Collision|LineTraceByChannel (LocalVariables|GetSpawnLocation) (- (LocalVariables|GetSpawnLocation) "0.000000,0.000000,1000.000000") "TraceTypeQuery1" false 0 "None"))
        (if _returnvalue
          (LocalVariables|SetSpawnLocation (.Location (Collision|BreakHitResult _outhit))))))
    (:then_1
      (bind _returnvalue_2 (Game|SpawnActorfromClass (Class|ItemObject|GetItemClass ItemObject) (Math|Transform|MakeTransform (LocalVariables|GetSpawnLocation) "0, 0, 0" "1.000000,1.000000,1.000000") "Undefined" 0 0))
      (Class|Item|SetItemObject _returnvalue_2 ItemObject))))