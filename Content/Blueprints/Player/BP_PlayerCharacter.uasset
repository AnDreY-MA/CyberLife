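; Player character Blueprint with a save-slot loader and a debug readout of damage taken.
; The SaveLoad function loads the BP_Saver object from slot "save1", or creates and saves a new one if none exists, then caches it in a variable.
; AnyDamage only prints the damage amount; no health logic is present, and the construction script is empty.
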(event Game|Damage|EventAnyDamage
  (params (Damage :type Float%20%28single-precision%29) (DamageType :type Damage%20Type%20Object%20Reference) (InstigatedBy :type Controller%20Object%20Reference) (DamageCauser :type Actor%20Object%20Reference))
  (Development|PrintString (Utilities|String|ToString(Float) Damage)))

(fn ConstructionScript)

(fn SaveLoad
  (bind _returnvalue (SaveGame|DoesSaveGameExist "save1"))
  (if _returnvalue
    (bind _returnvalue_2 (SaveGame|LoadGamefromSlot "save1"))
    (bind _asbp_saver (Utilities|Casting|CastToBP_Saver _returnvalue_2))
    (Variables|Default|SetBP%20Saver _asbp_saver)
    (else
      (bind _returnvalue_3 (SaveGame|CreateSaveGameObject "/Game/Blueprints/BP_Saver.BP_Saver_C"))
      (bind _output_get (Variables|Default|SetBP%20Saver _returnvalue_3))
      (SaveGame|SaveGametoSlot _output_get "save1"))))