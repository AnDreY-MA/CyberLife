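; BP_ItemObject is an item data object that exposes an item's dimensions, icon and class, with support for a rotated state.
; Rotate toggles a boolean flag, which IsRotated reports.
; That flag makes GetDimensions swap X and Y and GetIcon return a separate pre-rotated icon, so callers always receive values matching the current orientation.
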(fn BPGetDimensions
  (bind _bp_dimensions (Variables|Default|GetBP_Dimensions))
  (if (Variables|Default|GetBP_bRotated)
    (return (Utilities|Struct|MakeIntPoint (.y _bp_dimensions) (.x _bp_dimensions)))
    (else
      (return (Variables|Default|GetBP_Dimensions)))))

(fn BPGetIcon
  (return (select (Variables|Default|GetBP_bRotated) (Variables|Default|GetBP_IconRotated) (Variables|Default|GetBP_Icon))))

(fn BPGetItemClass
  (return (Variables|Default|GetBP_ItemClass)))

(fn BPRotate
  (Variables|Default|SetBP_bRotated (not (Variables|Default|GetBP_bRotated))))

(fn BPIsRotated
  (return (Variables|Default|GetBP_bRotated)))