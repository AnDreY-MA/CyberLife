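; BP_Mirror is an unfinished breakable mirror actor meant to shatter into fragment actors on impact.
; BreakOnImpact compares mesh speed and the dot product of velocity direction and impact normal against thresholds, then prints a debug string and fires the empty Break event.
; SpawnFragments spawns BP_MirrorFragments at the mesh transform, overrides the mirror's own mass and destroys it inside the loop.
; Nothing wired in the graph calls either function.
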(event Custom|Break)

(fn ConstructionScript)

(fn BreakonImpact
  (params (HitResult :type Hit%20Result%20Structure))
  (bind _staticmesh (Variables|Default|GetStaticMesh))
  (bind _returnvalue (Transformation|GetComponentVelocity _staticmesh))
  (if (and (> (Math|Vector|VectorLength _returnvalue) (Variables|Default|GetImpact%20Velocity%20Threshold)) (> (Math|Vector|DotProduct (Math|Vector|Normalize _returnvalue) (.ImpactNormal (Collision|BreakHitResult HitResult))) (Variables|Default|GetImpact%20Angle%20Threshold)))
    (Development|PrintString "Hello")
    (CallFunction|Break)))

(fn SpawnFragments
  (for _array_element (Variables|Default|GetFragments)
    (Game|SpawnActorfromClass "/Game/Blueprints/BP_MirrorFragments.BP_MirrorFragments_C" (Transformation|GetWorldTransform (Variables|Default|GetStaticMesh)) "Undefined" "OverrideRootScale" 0 0)
    (Class|PrimitiveComponent|SetMassOverrideinKg (Variables|Default|GetStaticMesh) "None" (Physics|GetMass (Variables|Default|GetStaticMesh)) true)
    (Actor|DestroyActor)))